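; Track checkpoint actor that scores SportsCar_Pawn cars as they progress along a spline.
; Construction rebuilds the spline by chaining the TraceActor's landscape spline mesh endpoints, then tiles it with evenly spaced overlap boxes.
; Overlaps award points only within a forward index window, allowing for lap wraparound and a car's first checkpoint.
; Helpers return a checkpoint's start transform and the interpolated spline distance nearest a location.
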(event Custom|OnBoxOverlap
  (params (OverlappedComponent :type Primitive%20Component%20Object%20Reference) (OtherActor :type Actor%20Object%20Reference) (OtherComp :type Primitive%20Component%20Object%20Reference) (OtherBodyIndex :type Integer) (bFromSweep :type Boolean) (SweepResult :type Hit%20Result%20Structure%20%28by%20ref%29))
  (bind _asbox_collision (Utilities|Casting|CastToBoxComponent OverlappedComponent))
  (bind _boxcomponents (Variables|Default|GetBoxComponents))
  (bind _returnvalue (Utilities|Array|FindItem _boxcomponents _asbox_collision))
  (bind _assports_car_pawn (Utilities|Casting|CastToSportsCar_Pawn OtherActor))
  (if (Math|Boolean|ORBoolean (or (and (< (- _returnvalue (Variables|/Game/VehicleTemplate/Blueprints/SportsCar/SportsCar_Pawn.SportsCar_Pawn_C|GetCheckpoint _assports_car_pawn)) 35) (> (- _returnvalue (Variables|/Game/VehicleTemplate/Blueprints/SportsCar/SportsCar_Pawn.SportsCar_Pawn_C|GetCheckpoint _assports_car_pawn)) 0)) (and (< (- _returnvalue (- (Variables|/Game/VehicleTemplate/Blueprints/SportsCar/SportsCar_Pawn.SportsCar_Pawn_C|GetCheckpoint _assports_car_pawn) (Utilities|Array|Length _boxcomponents))) 35) (> (- _returnvalue (- (Variables|/Game/VehicleTemplate/Blueprints/SportsCar/SportsCar_Pawn.SportsCar_Pawn_C|GetCheckpoint _assports_car_pawn) (Utilities|Array|Length _boxcomponents))) 0))) (and (== (Variables|/Game/VehicleTemplate/Blueprints/SportsCar/SportsCar_Pawn.SportsCar_Pawn_C|GetCheckpoint _assports_car_pawn) (- (Utilities|Array|Length _boxcomponents) 1)) (== _returnvalue 0)) (== (Variables|/Game/VehicleTemplate/Blueprints/SportsCar/SportsCar_Pawn.SportsCar_Pawn_C|GetCheckpoint _assports_car_pawn) -1))
    (Default|ScoreCheckpoint _assports_car_pawn _returnvalue 1e+01)))

(event EventBeginPlay)

(event Collision|EventActorBeginOverlap
  (params (OtherActor :type Actor%20Object%20Reference)))

(event EventTick
  (params (DeltaSeconds :type Float%20%28single-precision%29)))

(fn ConstructionScript
  (CallFunction|Setup))

(fn Setup
  (bind _traceactor (Variables|Default|GetTraceActor))
  (bind _splinepointtransforms (LocalVariables|GetSplinePointTransforms))
  (bind _splinepointtransforms_2 (LocalVariables|GetSplinePointTransforms))
  (bind _spline (Variables|Default|GetSpline))
  (bind _pointsize (Variables|Default|GetPointSize))
  (bind _boxcomponents (Variables|Default|GetBoxComponents))
  (bind _returnvalue (Transformation|GetActorTransform _traceactor))
  (bind _returnvalue_2 (Spline|GetSplineLength _spline))
  (bind (_x _y _z) (Math|Vector|BreakVector _pointsize))
  (Utilities|Array|Clear (LocalVariables|GetSplinePointTransforms))
  (Utilities|FlowControl|Sequence
    (:then_0
      (if (Utilities|IsValid _traceactor)
        (Transformation|SetActorTransform (Math|Transform|MakeTransform (.location _returnvalue) (.rotation _returnvalue) "1.000000,1.000000,1.000000"))
        (for _array_element (Actor|GetComponentsByClass _traceactor "/Script/Landscape.LandscapeSplinesComponent")
          (bind _returnvalue_3 (Class|LandscapeSplinesComponent|GetSplineMeshComponents _array_element))
          (bind _output_get (LocalVariables|SetSplines _returnvalue_3))
          (bind _output_get_2 (LocalVariables|SetLastPoint (+ (.Location (Math|Transform|BreakTransform (Transformation|GetRelativeTransform (Utilities|Array|Get(acopy) _output_get)))) (Math|Vector|RotateVector (SplineMesh|GetStartPosition (Utilities|Array|Get(acopy) _output_get)) (.Rotation (Math|Transform|BreakTransform (Transformation|GetRelativeTransform (Utilities|Array|Get(acopy) _output_get))))))))
          (Utilities|Array|Add _splinepointtransforms _output_get_2)
          (while (> (Utilities|Array|Length _output_get) 0)
            (for (_array_element_2 _array_index) _output_get
              (if (Utilities|Operators|EqualEqual (LocalVariables|GetLastPoint) (+ (.Location (Math|Transform|BreakTransform (Transformation|GetRelativeTransform _array_element_2))) (Math|Vector|RotateVector (SplineMesh|GetEndPosition _array_element_2) (.Rotation (Math|Transform|BreakTransform (Transformation|GetRelativeTransform _array_element_2))))) 1.0)
                (Utilities|Array|Add _splinepointtransforms (+ (.Location (Math|Transform|BreakTransform (Transformation|GetRelativeTransform _array_element_2))) (Math|Vector|RotateVector (SplineMesh|GetStartPosition _array_element_2) (.Rotation (Math|Transform|BreakTransform (Transformation|GetRelativeTransform _array_element_2))))))
                (LocalVariables|SetLastPoint (+ (.Location (Math|Transform|BreakTransform (Transformation|GetRelativeTransform _array_element_2))) (Math|Vector|RotateVector (SplineMesh|GetStartPosition _array_element_2) (.Rotation (Math|Transform|BreakTransform (Transformation|GetRelativeTransform _array_element_2))))))
                (Utilities|Array|RemoveItem (LocalVariables|GetSplines) _array_element_2 :!label _label)
                (elif (Utilities|Operators|EqualEqual (LocalVariables|GetLastPoint) (+ (.Location (Math|Transform|BreakTransform (Transformation|GetRelativeTransform _array_element_2))) (Math|Vector|RotateVector (SplineMesh|GetStartPosition _array_element_2) (.Rotation (Math|Transform|BreakTransform (Transformation|GetRelativeTransform _array_element_2))))) 1.0)
                  (Utilities|Array|Add _splinepointtransforms (+ (.Location (Math|Transform|BreakTransform (Transformation|GetRelativeTransform _array_element_2))) (Math|Vector|RotateVector (SplineMesh|GetEndPosition _array_element_2) (.Rotation (Math|Transform|BreakTransform (Transformation|GetRelativeTransform _array_element_2))))))
                  (LocalVariables|SetLastPoint (+ (.Location (Math|Transform|BreakTransform (Transformation|GetRelativeTransform _array_element_2))) (Math|Vector|RotateVector (SplineMesh|GetEndPosition _array_element_2) (.Rotation (Math|Transform|BreakTransform (Transformation|GetRelativeTransform _array_element_2))))))
                  (goto _label))))))
        (else
          (Development|PrintString "NoTrace")
          (Utilities|Array|Add :TargetArray _splinepointtransforms_2)
          (Utilities|Array|Add _splinepointtransforms_2 "200.000000,0,0"))))
    (:then_1
      (for _array_element_3 _boxcomponents
        (Components|DestroyComponent _array_element_3))
      (Utilities|Array|Clear _boxcomponents))
    (:then_2
      (Spline|SetSplinePoints _spline (LocalVariables|GetSplinePointTransforms) "Local" true)
      (bind _output_get_3 (LocalVariables|SetNumCheckPoints (Math|Float|Round (/ _returnvalue_2 _x))))
      (bind _output_get_4 (Variables|Default|SetPointSizeTrue (Math|Vector|MakeVector (/ _returnvalue_2 (Math|Conversions|ToFloat(Integer) _output_get_3)) _y _z)))
      (for _index (range 0 (- _output_get_3 1))
        (Development|PrintString (Utilities|String|ToString(Float) (.X (Math|Vector|BreakVector _output_get_4))))
        (bind _returnvalue_4 (AddComponent|AddBoxComponent false (Math|Transform|MakeTransform (+ (.Location (Math|Transform|BreakTransform (Spline|GetTransformatDistanceAlongSpline (Variables|Default|GetSpline) (+ (* _index (.X (Math|Vector|BreakVector _output_get_4))) (/ (.X (Math|Vector|BreakVector _output_get_4)) 2.0)) "Local" false))) (Math|Vector|RotateVector (Math|Vector|MakeVector 0.0 0.0 (/ (.z (Variables|Default|GetPointSizeTrue)) 2.0)) (.Rotation (Math|Transform|BreakTransform (Spline|GetTransformatDistanceAlongSpline (Variables|Default|GetSpline) (+ (* _index (.X (Math|Vector|BreakVector _output_get_4))) (/ (.X (Math|Vector|BreakVector _output_get_4)) 2.0)) "Local" false))))) (.Rotation (Math|Transform|BreakTransform (Spline|GetTransformatDistanceAlongSpline (Variables|Default|GetSpline) (+ (* _index (.X (Math|Vector|BreakVector _output_get_4))) (/ (.X (Math|Vector|BreakVector _output_get_4)) 2.0)) "Local" false))))))
        (Components|Box|SetBoxExtent _returnvalue_4 (* (Variables|Default|GetPointSizeTrue) "0.500000,0.500000,0.500000") true)
        (Collision|SetCollisionProfileName _returnvalue_4 "Checkpoint" true :!class /Script/Engine.PrimitiveComponent)
        (Development|SetHiddeninGame _returnvalue_4 false false)
        (Utilities|Array|Add (Variables|Default|GetBoxComponents) _returnvalue_4)
        (Collision|BindEventtoOnComponentBeginOverlap _returnvalue_4 (EventDispatchers|CreateEvent :!event Custom|OnBoxOverlap))))))

(fn GetStartTransform
  (params (Index :type Integer))
  (bind _boxcomponents (Variables|Default|GetBoxComponents))
  (bind _returnvalue (Utilities|Array|Length _boxcomponents))
  (bind _returnvalue_2 (Math|Integer|%(Integer) _returnvalue Index))
  (bind _output (Utilities|Array|Get(acopy) _boxcomponents _returnvalue_2))
  (bind _returnvalue_3 (Transformation|GetWorldTransform _output))
  (return (Math|Transform|MakeTransform (.location _returnvalue_3) (.rotation _returnvalue_3) "1.000000,1.000000,1.000000")))

(fn GetNearetDist
  (params (InLocation :type Vector))
  (bind _spline (Variables|Default|GetSpline))
  (bind _returnvalue (Class|SplineComponent|FindInputKeyClosesttoWorldLocation _spline InLocation))
  (bind _returnvalue_2 (Math|Float|Truncate _returnvalue))
  (bind _returnvalue_3 (Spline|GetDistanceAlongSplineatSplinePoint _spline _returnvalue_2))
  (return (+ _returnvalue_3 (* (- (Spline|GetDistanceAlongSplineatSplinePoint _spline (Math|Float|Truncate (+ _returnvalue 1.0))) _returnvalue_3) (- _returnvalue (Math|Conversions|ToFloat(Integer) _returnvalue_2))))))