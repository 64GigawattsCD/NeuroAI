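; Game mode that trains neural-network-driven sports cars on a checkpoint-spline track through neuroevolution at 4x time dilation.
; It loads the "Neuro" save's lineage, or seeds mutated random networks, and spawns one car per lobe at a shared random start.
; When all cars are gone or a timer expires, it records scores, then breeds, mutates, keeps survivors, saves and respawns.
; A looping timer points the camera at the top scorer.
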(event Custom|Reset
  (bind _array (Utilities|Array|MakeArray "DistSide" "DeltaHeading" "Speed" "DistSide" "DeltaHeadingPred"))
  (bind _cars (Variables|Default|GetCars))
  (bind _returnvalue (Utilities|Array|Length _array))
  (Utilities|Time|ClearandInvalidateTimerbyHandle (Variables|Default|GetMaxTime))
  (bind _returnvalue_2 (Utilities|Time|SetTimerbyEvent (delegate Custom|Reset) 9e+01))
  (Variables|Default|SetMaxTime _returnvalue_2)
  (if (Variables|Default|GetFirst)
    (Variables|Default|SetFirst false)
    (Utilities|FlowControl|Sequence :!label _label
      (:then_0
        (bind _returnvalue_3 (SaveGame|LoadGamefromSlot "Neuro"))
        (Utilities|IsValid _returnvalue_3 :!label _label_2
          (:Is%20Valid
            (bind _asbp_neuro_vehicle_save (Utilities|Casting|CastToBP_NeuroVehicleSave _returnvalue_3)
              (:then
                (bind _output_get (Variables|Default|SetSave _asbp_neuro_vehicle_save))
                (bind _returnvalue_4 (Class|NeuroAIBPLibrary|GetLatestGeneration (Variables|/Game/Neuro/BP_NeuroVehicleSave.BP_NeuroVehicleSave_C|GetLineage _output_get)))
                (bind _returnvalue_5 (Class|NeuroAIBPLibrary|GetGenerationLobes _returnvalue_4))
                (if (<= (Utilities|Array|Length _returnvalue_5) 0)
                  (bind _returnvalue_6 (SaveGame|CreateSaveGameObject "/Game/Neuro/BP_NeuroVehicleSave.BP_NeuroVehicleSave_C" :!label _label_3))
                  (Variables|Default|SetSave _returnvalue_6)
                  (bind _returnvalue_7 (Class|NeuroAIBPLibrary|GenerateRandomNeuroLobe _array (Utilities|Array|MakeArray "Steering" "Acceleration") 4 (* _returnvalue _returnvalue) "NAct_None" "NAct_RectLinear" "NAct_None"))
                  (for _index (range 0 59)
                    (bind _returnvalue_8 (Class|NeuroAIBPLibrary|MutateLobeSimple _returnvalue_7 3 3 0.2 0.02))
                    (Utilities|Array|Add (Variables|Default|GetFirstLobes) _returnvalue_8))
                  (bind _returnvalue_9 (Class|NeuroAIBPLibrary|SetGenerationLobes (Utilities|Struct|MakeNeuroGeneration) (Variables|Default|GetFirstLobes)))
                  (bind _returnvalue_10 (Class|NeuroAIBPLibrary|AppendGenerationtoLineage (Variables|/Game/Neuro/BP_NeuroVehicleSave.BP_NeuroVehicleSave_C|GetLineage _returnvalue_6) _returnvalue_9))
                  (Variables|/Game/Neuro/BP_NeuroVehicleSave.BP_NeuroVehicleSave_C|SetLineage (Variables|Default|GetSave) _returnvalue_10)
                  (SaveGame|SaveGametoSlot (Variables|Default|GetSave) "Neuro")))
              (:CastFailed
                (goto _label_2))))
          (:Is%20Not%20Valid
            (goto _label_3))))
      (:then_1
        (bind _returnvalue_11 (Class|NeuroAIBPLibrary|GetLatestGeneration (Variables|/Game/Neuro/BP_NeuroVehicleSave.BP_NeuroVehicleSave_C|GetLineage (Variables|Default|GetSave))))
        (bind _returnvalue_12 (Class|NeuroAIBPLibrary|GetGenerationLobes _returnvalue_11))
        (bind _spline (CallFunction|GetTrackActor))
        (bind _start (Default|GetStartTransform _spline (Math|Random|RandomInteger (- (Utilities|Array|Length (Variables|/Game/Track/BP_CheckpointSpline.BP_CheckpointSpline_C|GetBoxComponents _spline)) 1))))
        (for _array_element _returnvalue_12
          (bind _returnvalue_13 (Game|SpawnActorfromClass "/Game/VehicleTemplate/Blueprints/SportsCar/SportsCar_Pawn.SportsCar_Pawn_C" (Math|Transform|ComposeTransforms _start (Math|Transform|MakeTransform "0.000000,0.000000,125.000000")) "AlwaysSpawn" self 0))
          (Default|GetBrain _returnvalue_13 _array_element)
          (Utilities|Array|Add (Variables|Default|GetCars) _returnvalue_13)
          (Development|PrintString "Spawn"))))
    (else
      (Utilities|FlowControl|Sequence
        (:then_0
          (bind _returnvalue_14 (Class|NeuroAIBPLibrary|SetLastGenerationScores (Variables|/Game/Neuro/BP_NeuroVehicleSave.BP_NeuroVehicleSave_C|GetLineage (Variables|Default|GetSave)) (Variables|Default|GetScores)))
          (bind _returnvalue_15 (Class|NeuroAIBPLibrary|GetLatestGeneration _returnvalue_14))
          (bind _output_get_2 (Variables|Default|SetLastgen _returnvalue_15))
          (bind _returnvalue_16 (Class|NeuroAIBPLibrary|BreedNewGeneration _output_get_2 3 16))
          (bind _returnvalue_17 (Class|NeuroAIBPLibrary|MutateGenerationSimple _returnvalue_16 40 18 0.8 0.3))
          (bind _returnvalue_18 (Class|NeuroAIBPLibrary|SurviveLobes _returnvalue_17 _returnvalue_16 18))
          (bind _returnvalue_19 (Class|NeuroAIBPLibrary|SurviveLobes _output_get_2 _returnvalue_18 4))
          (bind _returnvalue_20 (Class|NeuroAIBPLibrary|AppendGenerationtoLineage _returnvalue_14 _returnvalue_19))
          (Variables|/Game/Neuro/BP_NeuroVehicleSave.BP_NeuroVehicleSave_C|SetLineage (Variables|Default|GetSave) _returnvalue_20)
          (SaveGame|SaveGametoSlot (Variables|Default|GetSave) "Neuro")
          (for _array_element_2 _cars
            (Utilities|IsValid _array_element_2
              (:Is%20Valid
                (Actor|DestroyActor _array_element_2))))
          (Utilities|Array|Clear _cars))
        (:then_1
          (goto _label))))))

(event Custom|UpdateLeader
  (Variables|Default|SetMaxPoints -1.0)
  (for _array_element (Variables|Default|GetCars)
    (Utilities|IsValid _array_element
      (:Is%20Valid
        (if (> (Variables|/Game/VehicleTemplate/Blueprints/SportsCar/SportsCar_Pawn.SportsCar_Pawn_C|GetTotalPoints _array_element) (Variables|Default|GetMaxPoints))
          (Variables|Default|SetMaxPoints (Variables|/Game/VehicleTemplate/Blueprints/SportsCar/SportsCar_Pawn.SportsCar_Pawn_C|GetTotalPoints _array_element))
          (Variables|Default|SetFollow _array_element)))))
  (Utilities|IsValid (Variables|Default|GetFollow)
    (:Is%20Valid
      (Game|Player|SetViewTargetwithBlend (Game|GetPlayerController 0) (Variables|Default|GetFollow) 0.5 "VTBlend_Linear" 0.0 false))))

(event EventBeginPlay
  (Utilities|Time|SetTimerbyEvent (delegate Custom|UpdateLeader) 1.0 true)
  (Utilities|Time|SetGlobalTimeDilation 4.0))

(event EventTick
  (params (DeltaSeconds :type Float%20%28single-precision%29))
  (bind _scores (Variables|Default|GetScores))
  (if (Variables|Default|GetNoReset)
    (Variables|Default|SetNoReset false)
    (for (_array_element _array_index) (Variables|Default|GetCars)
      (Utilities|IsValid _array_element
        (:Is%20Valid
          (Utilities|Array|SetArrayElem _scores _array_index (Variables|/Game/VehicleTemplate/Blueprints/SportsCar/SportsCar_Pawn.SportsCar_Pawn_C|GetTotalPoints _array_element) true)
          (Variables|Default|SetNoReset true))
        (:Is%20Not%20Valid
          (Utilities|Array|SetArrayElem _scores _array_index 0.0 true))))
    (else
      (CallFunction|Reset)
      (Variables|Default|SetNoReset true))))

(fn ConstructionScript)

(fn GetTrackActor
  (bind _returnvalue (Actor|GetActorOfClass "/Game/Track/BP_CheckpointSpline.BP_CheckpointSpline_C"))
  (return _returnvalue))